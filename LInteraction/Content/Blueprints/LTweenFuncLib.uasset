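; Blueprint function library of LTween helpers for transform animation and yoyo timing.
; LocalTransformTo builds a sequence running local position, shortest-path rotation and scale tweens in parallel, optionally jumping to a start time.
; GetYoyoDuration returns elapsed plus leftover time while tweening, otherwise the full duration.
; It also updates the leftover time by reference, carrying it between calls, with optional debug printing.
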(fn LocalTransformto
  (params (target :type Scene%20Component%20Object%20Reference) (EndTransform :type Transform) (Duration :type Float%20%28single-precision%29) (Delay :type Float%20%28single-precision%29) (StartAt :type Float%20%28double-precision%29) (Ease :type ELTweenEase%20Enum :default "OutCubic"))
  (bind _returnvalue (Class|LTweenBPLibrary|CreateSequence target))
  (bind _returnvalue_2 (Class|LTweenBPLibrary|LocalPositionto target (.location EndTransform) Duration Delay Ease))
  (Class|LTweenerSequence|Insert _returnvalue _returnvalue 0.0 _returnvalue_2)
  (bind _returnvalue_3 (Class|LTweenBPLibrary|LocalRotatorto target (.rotation EndTransform) true Duration Delay Ease))
  (Class|LTweenerSequence|Insert _returnvalue _returnvalue 0.0 _returnvalue_3)
  (bind _returnvalue_4 (Class|LTweenBPLibrary|LocalScaleto target (.scale EndTransform) Duration Delay Ease))
  (Class|LTweenerSequence|Insert _returnvalue _returnvalue 0.0 _returnvalue_4)
  (if (> StartAt 0.0)
    (Class|LTweener|Goto _returnvalue StartAt))
  (return _returnvalue))

(fn GetYoyoDuration
  (params (Target :type L%20Tweener%20Object%20Reference) (LeftTime :type Float%20%28double-precision%29%20%28by%20ref%29) (Duration :type Float%20%28double-precision%29) (Debug :type Boolean))
  (LocalVariables|Set_Duration Duration)
  (bind _output_get (LocalVariables|SetbIsTween (Class|LTweenBPLibrary|IsTweening Target Target)))
  (Utilities|FlowControl|Sequence
    (:then_0
      (if _output_get
        (bind _output_get_2 (LocalVariables|SetYoyoTime (+ (Class|LTweener|GetElapsedTime Target) LeftTime)))
        (|SetBy-RefVar LeftTime (- (LocalVariables|Get_Duration) _output_get_2))
        (else
          (|SetBy-RefVar LeftTime 0.0)
          (LocalVariables|SetYoyoTime (LocalVariables|Get_Duration)))))
    (:then_1
      (if Debug
        (Development|PrintString 0 (Utilities|String|Append "YoyoDuration:" (Utilities|String|ToString(Float) (LocalVariables|GetYoyoTime)) "/" (Utilities|String|ToString(Float) (LocalVariables|Get_Duration))) true true "(R=0.000000,G=0.660000,B=1.000000,A=1.000000)" 2.0 "GetYoyoDuration")))
    (:then_2
      (return (LocalVariables|GetYoyoTime) (LocalVariables|GetbIsTween)))))