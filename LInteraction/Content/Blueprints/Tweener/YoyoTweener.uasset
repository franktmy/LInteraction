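; YoyoTweener is a scene component that tweens its relative transform back and forth between a start and an end transform.
; A yoyo helper flips or reverts direction, then drives an LTween local-transform tween with easing and fires forward, backward, play or skip callbacks.
; Transacted editor functions snap to either endpoint or capture one from the component or a TweenActor relative to the owner.
; BeginPlay and Reset restore the configured endpoint.
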(event EventBeginPlay
  (Transformation|SetRelativeTransform (Getter|GetCurrentTransform) false false)
  (|CallParentFunction))

(event Custom|Yoyo
  ;[0.15 0.15 0.15 0.5] TweenYoyo
  (bind (_yoyoduration _isforward) (Utilities|LTweenYoyo (Variables|Default|GetLTweener) (Variables|Default|GetDuration) (Variables|Default|GetbCurrentAtEnd) (Variables|Default|GetbLastAtEnd) (Variables|Default|GetDebug))
    (:DoForward
      (CallFunction|DoForward)
      (bind _lsequence (CallFunction|LocalTransformto self (Math|Transform|SelectTransform (Variables|Default|GetEndTransform) (Variables|Default|GetStartTransform) _isforward) _yoyoduration 0.0 0.0 (Variables|Default|GetEase) :!label _label))
      (Variables|Default|SetLTweener _lsequence))
    (:DoBackward
      (CallFunction|DoBackward)
      (goto _label))
    (:Skip
      (CallFunction|DoSkip))))

(event Custom|DoForward
  ;[0.15 0.15 0.15 0.5] DoTween
  (Default|CallOnDoForward)
  (Default|CallOnPlay))

(event Custom|DoBackward
  ;[0.15 0.15 0.15 0.5] DoTween
  (Default|CallOnDoBackward)
  (Default|CallOnPlay))

(event Custom|PlayForward
  (params (Revert :type Boolean))
  ;[0.15 0.15 0.15 0.5] TweenYoyo
  (if Revert
    (Utilities|LTweenYoyo (Variables|Default|GetLTweener) (Variables|Default|GetDuration) (Variables|Default|GetbCurrentAtEnd) (Variables|Default|GetbLastAtEnd) (Variables|Default|GetDebug)) ; enters at Revert
    (else
      (Utilities|LTweenYoyo (Variables|Default|GetLTweener) (Variables|Default|GetDuration) (Variables|Default|GetbCurrentAtEnd) (Variables|Default|GetbLastAtEnd) (Variables|Default|GetDebug)) ; enters at Play
    )))

(event Custom|DoSkip
  ;[0.15 0.15 0.15 0.5] DoTween
  (Default|CallOnSkip))

(fn ToStart
  (Class|KismetSystemLibrary|BeginTransaction "ToStart" "ToStart")
  (Transactions|TransactObject self)
  (Transformation|SetRelativeTransform (Variables|Default|GetStartTransform) false false)
  (CallFunction|Align)
  (Variables|Default|SetbCurrentAtEnd false)
  (Class|KismetSystemLibrary|EndTransaction))

(fn ToEnd
  (Class|KismetSystemLibrary|BeginTransaction "ToEnd" "ToStart")
  (Transactions|TransactObject self)
  (Transformation|SetRelativeTransform (Variables|Default|GetEndTransform) false false)
  (CallFunction|Align)
  (Variables|Default|SetbCurrentAtEnd true)
  (Class|KismetSystemLibrary|EndTransaction))

(fn CopytoStart
  (Class|KismetSystemLibrary|BeginTransaction "CopyToStart" "CopyToStart")
  (Transactions|TransactObject self)
  (Variables|Default|SetStartTransform (Getter|SelectTreansform))
  (Class|KismetSystemLibrary|EndTransaction))

(fn CopytoEnd
  (Class|KismetSystemLibrary|BeginTransaction "CopyToStart" "CopyToEnd")
  (Transactions|TransactObject self)
  (Variables|Default|SetEndTransform (Getter|SelectTreansform))
  (Class|KismetSystemLibrary|EndTransaction))

(fn GetCurrentTransform
  (return (Math|Transform|SelectTransform (Variables|Default|GetEndTransform) (Variables|Default|GetStartTransform) (Variables|Default|GetbCurrentAtEnd))))

(fn SelectTreansform
  (Utilities|IsValid (Variables|Default|GetTweenActor)
    (:Is%20Valid
      (return (Math|Transform|SelectTransform (Math|Transform|MakeRelativeTransform (Transformation|GetActorTransform (Variables|Default|GetTweenActor)) (Transformation|GetActorTransform (Components|GetOwner))) (Transformation|GetRelativeTransform) (Utilities|IsValid (Variables|Default|GetTweenActor)))))
    (:Is%20Not%20Valid
      (return (Transformation|GetRelativeTransform)))))

(fn Play
  (CallFunction|Yoyo)
  (return (Variables|Default|GetLTweener)))

(fn Reset
  (|CallParentFunction)
  (Transformation|SetRelativeTransform (Getter|GetCurrentTransform) false false))