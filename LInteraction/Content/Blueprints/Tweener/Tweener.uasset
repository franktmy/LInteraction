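; Tweener is a scene component that carries a TweenActor and exposes playback controls for an LTweener, likely as a base for specific tweens.
; On BeginPlay it snap-attaches a valid TweenActor to itself, so the actor follows the component's transform.
; Align moves that actor to the component's world transform as an undoable transaction.
; Play only returns the LTweener, Pause and Resume forward to it, and Reset is an empty stub.
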(event EventBeginPlay
  (bind _tweenactor (Variables|Default|GetTweenActor))
  (Utilities|IsValid _tweenactor
    (:Is%20Valid
      (Transformation|AttachComponentToComponent _tweenactor self "None" "SnapToTarget" "SnapToTarget" "SnapToTarget" true))))

(fn Play
  (return (Variables|Default|GetLTweener)))

(fn Align
  (Transactions|TransactObject (Variables|Default|GetTweenActor))
  (Transformation|SetActorTransform (Variables|Default|GetTweenActor) (Transformation|GetWorldTransform)))

(fn Pause
  (Class|LTweener|Pause (Variables|Default|GetLTweener)))

(fn Resume
  (Class|LTweener|Resume (Variables|Default|GetLTweener)))

(fn Reset)