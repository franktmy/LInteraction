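; Incremental tweener Blueprint that animates its own relative transform by a delta offset using LTween.
; Play stops any running tween, then starts and returns a local transform tween using the configured duration and ease.
; GetTargetTransform adds the delta's location, rotation (per axis) and scale to the current relative transform, so each play steps from wherever it currently sits.
; BeginPlay, Tick and OnCycleComplete contain no logic.
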(event Custom|OnCycleComplete)

(event EventBeginPlay)

(event EventTick
  (params (DeltaSeconds :type Float%20%28single-precision%29)))

(fn Play
  (Class|LTweenBPLibrary|KillifIsTweening (Variables|Default|GetLTweener))
  (bind _lsequence (CallFunction|LocalTransformto self (CallFunction|GetTargetTransform) (Variables|Default|GetDuration) 0.0 0.0 (Variables|Default|GetEase)))
  (bind _output_get (Variables|Default|SetLTweener _lsequence))
  (return _output_get))

(fn GetTargetTransform
  (bind _returnvalue (Transformation|GetRelativeTransform))
  (bind _deltatransform (Variables|Default|GetDeltaTransform))
  (return (Math|Transform|MakeTransform (+ (.location _returnvalue) (.location _deltatransform)) (Math|Rotator|MakeRotator (+ (.roll (.rotation _returnvalue)) (.roll (.rotation _deltatransform))) (+ (.pitch (.rotation _returnvalue)) (.pitch (.rotation _deltatransform))) (+ (.yaw (.rotation _returnvalue)) (.yaw (.rotation _deltatransform)))) (+ (.scale _returnvalue) (.scale _deltatransform)))))